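; BP_Pickup_Battery is an interactable battery pickup that shows a "Pick Up" prompt.
; On interaction it casts the interacting actor to BP_FirstPersonCharacter, calls its PickupBattery, plays a 2D pickup sound and destroys itself.
; CanInteract returns false while the actor is being destroyed, and Interact checks it before doing anything.
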(event `/Game/Interaction/BPI_Interactable.Interact`
  (params (InteractingActor :type "Actor Object Reference"))
  (bind _returnvalue (`self.CanInteract`))
  (if _returnvalue
    (bind _asbp_first_person_character (cast `/Game/FirstPerson/Blueprints/BP_FirstPersonCharacter` InteractingActor))
    (`/Game/FirstPerson/Blueprints/BP_FirstPersonCharacter.PickupBattery` _asbp_first_person_character)
    (`GameplayStatics.PlaySound2D` "/Game/Sounds/BatteryPickup.BatteryPickup" 1.0 1.0 0.0 null null)
    (`self.K2_DestroyActor`)))

(fn `CanInteract`
  (returns (ReturnValue :type Boolean))
  (return (not (`self.IsActorBeingDestroyed`))))

(fn `GetInteractText`
  (returns (ReturnValue :type Text))
  (return "Pick Up"))

(fn `UserConstructionScript`)