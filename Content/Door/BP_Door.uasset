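; BP_Door is an interactable door that takes batteries from the player and shows its count, with no opening logic.
; Interact calls AddBattery, which consumes a player battery while below BatteryMax and updates the BatteryCounter text.
; CollisionBox overlap sets IsInRange for CanInteract, but end overlap compares OverlappedComponent, not OtherActor, to the player pawn.
; RemoveBattery returns a battery to the player but is not called here.
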(event `self.ReceiveBeginPlay`
  (bind _asbp_first_person_character (cast `/Game/FirstPerson/Blueprints/BP_FirstPersonCharacter` (`GameplayStatics.GetPlayerCharacter` 0)))
  (set `self.BP_FirstPersonCharacter` _asbp_first_person_character)
  (`self.SetBatteryCountText`))

(event `self.CollisionBox.OnComponentBeginOverlap`
  (params (OverlappedComponent :type "PrimitiveComponent Object Reference") (OtherActor :type "Actor Object Reference") (OtherComp :type "PrimitiveComponent Object Reference") (OtherBodyIndex :type Integer) (bFromSweep :type Boolean) (SweepResult :type "HitResult Structure (by ref)"))
  (if (== OtherActor (`GameplayStatics.GetPlayerPawn` 0))
    (set `self.IsInRange` true)))

(event `self.CollisionBox.OnComponentEndOverlap`
  (params (OverlappedComponent :type "PrimitiveComponent Object Reference") (OtherActor :type "Actor Object Reference") (OtherComp :type "PrimitiveComponent Object Reference") (OtherBodyIndex :type Integer))
  (if (== OverlappedComponent (`GameplayStatics.GetPlayerPawn` 0))
    (set `self.IsInRange` false)))

(event `/Game/Interaction/BPI_Interactable.Interact`
  (params (InteractingActor :type "Actor Object Reference"))
  (`self.AddBattery`))

(fn `AddBattery`
  (bind _returnvalue (`/Game/FirstPerson/Blueprints/BP_FirstPersonCharacter.HasBattery` (`self.BP_FirstPersonCharacter`)))
  (if (and _returnvalue (< (`self.BatteryCount`) (`self.BatteryMax`)))
    (`/Game/FirstPerson/Blueprints/BP_FirstPersonCharacter.UseBattery` (`self.BP_FirstPersonCharacter`))
    (set `self.BatteryCount` (+ (`self.BatteryCount`) 1))
    (`self.SetBatteryCountText`)))

(fn `CanInteract`
  (returns (ReturnValue :type Boolean))
  (return (`self.IsInRange`)))

(fn `GetInteractText`
  (returns (ReturnValue :type Text))
  (return ""))

(fn `RemoveBattery`
  ;[1 0 0] Would need another interaction button to remove battery
  (if (> (`self.BatteryCount`) 0)
    (set `self.BatteryCount` (- (`self.BatteryCount`) 1))
    (`/Game/FirstPerson/Blueprints/BP_FirstPersonCharacter.PickupBattery` (`self.BP_FirstPersonCharacter`))
    (`self.SetBatteryCountText`)))

(fn `SetBatteryCountText`
  (`TextRenderComponent.K2_SetText` (`self.BatteryCounter`) (`|FormatText` "{Count}/{Max}" (`self.BatteryCount`) (`self.BatteryMax`))))

(fn `UserConstructionScript`)