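; BP_LightControlPanel is an interactable panel that toggles the battery in a linked light source.
; Interact calls RemoveBattery or InsertBattery on the BPLightSource reference, depending on its HasBattery state, and GetInteractText shows the matching prompt.
; Collision box overlaps with the player pawn set IsInRange, which CanInteract returns to allow interaction only up close.
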(event `/Game/Interaction/BPI_Interactable.Interact`
  (params (InteractingActor :type "Actor Object Reference"))
  (if (`/Game/LevelPrototyping/Meshes/BP_LightSource.HasBattery` (`self.BP_LightSource`))
    (`/Game/LevelPrototyping/Meshes/BP_LightSource.RemoveBattery` (`self.BP_LightSource`))
    (else
      (`/Game/LevelPrototyping/Meshes/BP_LightSource.InsertBattery` (`self.BP_LightSource`)))))

(event `self.CollisionBox.OnComponentBeginOverlap`
  (params (OverlappedComponent :type "PrimitiveComponent Object Reference") (OtherActor :type "Actor Object Reference") (OtherComp :type "PrimitiveComponent Object Reference") (OtherBodyIndex :type Integer) (bFromSweep :type Boolean) (SweepResult :type "HitResult Structure (by ref)"))
  (if (== OtherActor (`GameplayStatics.GetPlayerPawn` 0))
    (set `self.IsInRange` true)))

(event `self.CollisionBox.OnComponentEndOverlap`
  (params (OverlappedComponent :type "PrimitiveComponent Object Reference") (OtherActor :type "Actor Object Reference") (OtherComp :type "PrimitiveComponent Object Reference") (OtherBodyIndex :type Integer))
  (if (== OtherActor (`GameplayStatics.GetPlayerPawn` 0))
    (set `self.IsInRange` false)))

(fn `CanInteract`
  (returns (ReturnValue :type Boolean))
  (return (`self.IsInRange`)))

(fn `GetInteractText`
  (returns (ReturnValue :type Text))
  (if (`/Game/LevelPrototyping/Meshes/BP_LightSource.HasBattery` (`self.BP_LightSource`))
    (return "Remove Battery")
    (else
      (return "Insert Battery"))))

(fn `UserConstructionScript`)